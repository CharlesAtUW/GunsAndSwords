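; BP_Gun is a gun actor that manages magazine and standby ammo, firing feedback, reloading and damage values.
; Fire spends a round and triggers particles and a gunshot sound, or plays an empty-gun sound when the magazine is empty.
; Reload moves as much standby ammo as fits into the magazine and plays a cocking sound.
; GetDamage returns headshot or normal damage; the gun itself performs no hit detection.
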(event `Fire`
  (if (`self.CanShoot`)
    (`/Engine/EditorBlueprintResources/StandardMacros.DecrementInt` (`self.CurrentAmmo`)
      (:`  `
        (`ActorComponent.Activate` (`self.GunfireParticles`) true)
        (`AudioComponent.Play` (`self.GunfireSound`) (`self.ShootSoundStartTime`))))
    (else
      (`AudioComponent.Play` (`self.EmptyGunSound`) (`self.EmptySoundStartTime`)))))

(fn `CanReload`
  (returns (CanReload :type Boolean))
  (return (and (!= (`self.MagazineSize`) (`self.CurrentAmmo`)) (!= (`self.StandbyAmmo`) 0))))

(fn `CanShoot`
  (returns (CanShoot :type Boolean))
  (return (!= (`self.CurrentAmmo`) 0)))

(fn `GetDamage`
  (params (Headshot :type Boolean))
  (returns (Damage :type "Float (double-precision)"))
  (return (`KismetMathLibrary.SelectFloat` (`self.HeadshotDamage`) (`self.ShootDamage`) Headshot)))

(fn `Reload`
  (locals (ToReplenish :type Integer))
  (if (`self.CanReload`)
    (bind _output_get (set `local.ToReplenish` (`KismetMathLibrary.Min` (- (`self.MagazineSize`) (`self.CurrentAmmo`)) (`self.StandbyAmmo`))))
    (set `self.StandbyAmmo` (- (`self.StandbyAmmo`) _output_get))
    (set `self.CurrentAmmo` (+ (`self.CurrentAmmo`) (`local.ToReplenish`)))
    (`AudioComponent.Play` (`self.GunCockSound`) (`self.GunCockSoundStartTime`))))

(fn `UserConstructionScript`)