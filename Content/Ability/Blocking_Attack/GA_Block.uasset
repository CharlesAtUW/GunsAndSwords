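; Gameplay ability for the third-person character's block, with a timed parry window.
; On activation it commits, disables character movement and plays a montage.
; Parry-window open and close gameplay events add and remove loose, non-replicated parry tags.
; Cancel input or montage interruption restores walking, clears block and parry tags and ends the ability; normal montage completion does not end it.
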(event `self.K2_ActivateAbility`
  (bind _asbp_third_person_character_1 (cast `/Game/ThirdPerson/Blueprints/BP_ThirdPersonCharacter1` (`self.GetAvatarActorFromActorInfo`)))
  (`self.K2_CommitAbility`)
  (bind _charactermovement (`Character.CharacterMovement` _asbp_third_person_character_1))
  (`CharacterMovementComponent.SetMovementMode` _charactermovement "MOVE_None" 0)
  (`AbilityTask_PlayMontageAndWait.CreatePlayMontageAndWaitProxy` "None" (`self.Montage to Play`) 1.0 "None"
    (:`then`
      (`AbilityTask_WaitGameplayEvent.WaitGameplayEvent` (struct :`TagName` "Player.Block.ParryWindowOpen") null
        (:`then`
          (`AbilityTask_WaitGameplayEvent.WaitGameplayEvent` (struct :`TagName` "Player.Block.ParryWindowClose") null
            (:`then`
              (`AbilityTask_WaitCancel.WaitCancel`
                (:`OnCancel`
                  (`CharacterMovementComponent.SetMovementMode` _charactermovement "MOVE_Walking" 0 :!label _label)
                  (`AbilitySystemBlueprintLibrary.RemoveLooseGameplayTags` (`self.GetAvatarActorFromActorInfo`) (`self.Gameplay Tags`))
                  (`AbilitySystemBlueprintLibrary.RemoveLooseGameplayTags` (`self.GetAvatarActorFromActorInfo`) (`self.Parry Tags`))
                  (`self.K2_EndAbility`))))
            (:`EventReceived`
              (`AbilitySystemBlueprintLibrary.RemoveLooseGameplayTags` (`self.GetAvatarActorFromActorInfo`) (`self.Parry Tags`)))))
        (:`EventReceived`
          (`AbilitySystemBlueprintLibrary.AddLooseGameplayTags` (`self.GetAvatarActorFromActorInfo`) (`self.Parry Tags`)))))
    (:`OnInterrupted`
      (goto _label))))

(event `self.K2_OnEndAbility`
  (params (bWasCancelled :type Boolean))
  (`KismetSystemLibrary.PrintString` "Jump Attack Ended"))