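; Gameplay ability for the third attack of Combo02, which commits and plays an attack montage.
; It starts three gameplay event waits in parallel alongside the montage.
; Attack window open and close events add and remove a non-replicated loose tag on the avatar.
; The combo window end event clears the combo window tag and is the only wired path that ends the ability, with debug prints marking the end.
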(event `self.K2_ActivateAbility`
  (`self.K2_CommitAbility`)
  (`AbilityTask_PlayMontageAndWait.CreatePlayMontageAndWaitProxy` "None" (`self.Montage to Play`)
    (:`then`
      (`AbilityTask_WaitGameplayEvent.WaitGameplayEvent` (struct :`TagName` "Player.AttackWindowOpen") null
        (:`then`
          (`AbilityTask_WaitGameplayEvent.WaitGameplayEvent` (struct :`TagName` "Player.AttackWindowClose") null
            (:`then`
              (`AbilityTask_WaitGameplayEvent.WaitGameplayEvent` (struct :`TagName` "Event.ComboWindowEnd") null
                (:`EventReceived`
                  (`KismetSystemLibrary.PrintString` "Combo 3 Window End" true true (struct :`R` 1.0 :`G` 0.027451 :`A` 1.0))
                  (`AbilitySystemBlueprintLibrary.RemoveLooseGameplayTags` (`self.GetAvatarActorFromActorInfo`) (`self.ComboWindowTag`))
                  (`self.K2_EndAbility`))))
            (:`EventReceived`
              (`AbilitySystemBlueprintLibrary.RemoveLooseGameplayTags` (`self.GetAvatarActorFromActorInfo`) (`self.Attack Window Tag`)))))
        (:`EventReceived`
          (`AbilitySystemBlueprintLibrary.AddLooseGameplayTags` (`self.GetAvatarActorFromActorInfo`) (`self.Attack Window Tag`)))))))

(event `self.K2_OnEndAbility`
  (params (bWasCancelled :type Boolean))
  (`KismetSystemLibrary.PrintString` "Combo 3 Ended"))