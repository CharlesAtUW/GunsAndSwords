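; Gameplay Ability for a non-combo attack that commits, plays a montage and ends when it completes or is cancelled.
; Alongside the montage, it waits for the Player.AttackWindowOpen and AttackWindowClose gameplay events to add and remove a non-replicated loose attack-window tag on the avatar.
; OnEndAbility also removes the tag, so the window does not outlive the ability.
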(event `self.K2_ActivateAbility`
  (`self.K2_CommitAbility`)
  (`AbilityTask_PlayMontageAndWait.CreatePlayMontageAndWaitProxy` "None" (`self.Montage to Play`)
    (:`then`
      (`AbilityTask_WaitGameplayEvent.WaitGameplayEvent` (struct :`TagName` "Player.AttackWindowOpen") null
        (:`then`
          (`AbilityTask_WaitGameplayEvent.WaitGameplayEvent` (struct :`TagName` "Player.AttackWindowClose") null
            (:`EventReceived`
              (`AbilitySystemBlueprintLibrary.RemoveLooseGameplayTags` (`self.GetAvatarActorFromActorInfo`) (`self.AttackWindowTag`)))))
        (:`EventReceived`
          (`AbilitySystemBlueprintLibrary.AddLooseGameplayTags` (`self.GetAvatarActorFromActorInfo`) (`self.AttackWindowTag`)))))
    (:`OnCompleted`
      (`self.K2_EndAbility` :!label _label))
    (:`OnCancelled`
      (goto _label))))

(event `self.K2_OnEndAbility`
  (params (bWasCancelled :type Boolean))
  (`AbilitySystemBlueprintLibrary.RemoveLooseGameplayTags` (`self.GetAvatarActorFromActorInfo`) (`self.AttackWindowTag`)))